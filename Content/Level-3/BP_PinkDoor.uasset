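; BP_PinkDoor is a key-locked sliding door for Level-3.
; A box overlap caches the third-person character, whose HasKey flag gates the Interact event.
; Each permitted interaction alternates through a FlipFlop between playing and reversing a timeline that lerps the door mesh along its relative Y axis.
; A PickUpKey event sets HasKey on that cached character.
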(event OnComponentBeginOverlap(Box)
  (params (OverlappedComponent :type Primitive%20Component%20Object%20Reference) (OtherActor :type Actor%20Object%20Reference) (OtherComp :type Primitive%20Component%20Object%20Reference) (OtherBodyIndex :type Integer) (bFromSweep :type Boolean) (SweepResult :type Hit%20Result%20Structure%20%28by%20ref%29))
  (bind _asbp_third_person_character (Utilities|Casting|CastToBP_ThirdPersonCharacter OtherActor)))

(event EventInteract
  (if (Variables|/Game/ThirdPerson/Blueprints/BP_ThirdPersonCharacter.BP_ThirdPersonCharacter_C|GetHasKey? (stale OnComponentBeginOverlap(Box) _asbp_third_person_character))
    (Utilities|FlowControl|FlipFlop
      (:A
        (bind _dooropen (Timeline|Dooranim1 Play)
          (:Update
            (Transformation|SetRelativeLocation (Variables|Default|GetSM_Door1) (Math|Vector|MakeVector 0.0 (Math|Float|Lerp 0.0 9e+01 _dooropen) 0.0) false false))))
      (:B
        (Timeline|Dooranim1 Reverse)))))

(event EventPickUpKey
  (Variables|/Game/ThirdPerson/Blueprints/BP_ThirdPersonCharacter.BP_ThirdPersonCharacter_C|SetHasKey? (stale OnComponentBeginOverlap(Box) _asbp_third_person_character) true))

(fn ConstructionScript)