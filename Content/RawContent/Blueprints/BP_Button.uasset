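; BP_Button is an interactable puzzle button that opens its DoorWay when all lightable torches are lit.
; At BeginPlay it caches every BP_Lightable in the level.
; On Interact it compares the guard character's GuardLightsActive count to the torch total, opening the door on a match.
; Otherwise it resets the puzzle by swapping each lamp to the unlit material and hiding its light and fire effect.
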(event EventInteract
  (bind _torches (Variables|Default|GetTorches))
  (bind _returnvalue (Actor|GetActorOfClass "/Game/ThirdPerson/Blueprints/BP_GuardCharacter.BP_GuardCharacter_C"))
  (if (== (Variables|/Game/ThirdPerson/Blueprints/BP_GuardCharacter.BP_GuardCharacter_C|GetGuardLightsActive _returnvalue) (Utilities|Array|Length _torches))
    (Default|DoorOpen (Variables|Default|GetDoorWay))
    (else
      ;[0.15 0.15 0.15 0.5] Reset Puzzle
      (for _array_element _torches
        (Rendering|Material|SetMaterial (Variables|/Game/RawContent/Blueprints/BP_Lightable.BP_Lightable_C|GetLamp _array_element) 1 "/Game/Materials/M_Unlit.M_Unlit")
        (Rendering|SetVisibility (Variables|/Game/RawContent/Blueprints/BP_Lightable.BP_Lightable_C|GetPointLight _array_element) false false)
        (Rendering|SetVisibility (Variables|/Game/RawContent/Blueprints/BP_Lightable.BP_Lightable_C|GetNS_Stylish_Fire_4 _array_element) false false)))))

(event EventBeginPlay
  (bind _outactors (Actor|GetAllActorsOfClass "/Game/RawContent/Blueprints/BP_Lightable.BP_Lightable_C"))
  (Variables|Default|SetTorches _outactors))

(fn ConstructionScript)