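; BP_Lightable is an interactable lamp that forms one step of an ordered lighting sequence tracked on BP_GuardCharacter.
; Interacting while unlit shows its point light and fire effect and swaps the lamp material.
; A matching SequenceNumber increments the guard's GuardLightsActive counter, while a wrong one zeroes it.
; Reset hides the light and restores the unlit material, but leaves the fire effect untouched.
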(event EventInteract
  (bind _pointlight (Variables|Default|GetPointLight))
  (if (not (Rendering|IsVisible _pointlight))
    (Rendering|SetVisibility _pointlight true false)
    (Rendering|Material|SetMaterial (Variables|Default|GetLamp) 1 "/Game/Fab/Street_lighting_torch/street_lighting_torch/Materials/Material_001.Material_001")
    (Rendering|SetVisibility (Variables|Default|GetNS_Stylish_Fire_4) true false)
    (if (== (Variables|/Game/ThirdPerson/Blueprints/BP_GuardCharacter.BP_GuardCharacter_C|GetGuardLightsActive (stale EventBeginPlay _returnvalue)) (Variables|Default|GetSequenceNumber))
      (bind _returnvalue (Actor|GetActorOfClass "/Game/ThirdPerson/Blueprints/BP_GuardCharacter.BP_GuardCharacter_C"))
      (bind _result (Math|Integer|IncrementInt (Variables|/Game/ThirdPerson/Blueprints/BP_GuardCharacter.BP_GuardCharacter_C|GetGuardLightsActive _returnvalue))
        (:%20%20
          (Variables|/Game/ThirdPerson/Blueprints/BP_GuardCharacter.BP_GuardCharacter_C|SetGuardLightsActive _returnvalue _result)))
      (else
        (bind _returnvalue_2 (Actor|GetActorOfClass "/Game/ThirdPerson/Blueprints/BP_GuardCharacter.BP_GuardCharacter_C"))
        (Variables|/Game/ThirdPerson/Blueprints/BP_GuardCharacter.BP_GuardCharacter_C|SetGuardLightsActive _returnvalue_2 0)))))

(event EventBeginPlay
  (bind _returnvalue (Actor|GetActorOfClass "/Game/ThirdPerson/Blueprints/BP_GuardCharacter.BP_GuardCharacter_C")))

(fn ConstructionScript)

(fn Reset
  (Rendering|SetVisibility (Variables|Default|GetPointLight) false false)
  (Rendering|Material|SetMaterial (Variables|Default|GetLamp) 1 "/Game/Materials/M_Unlit.M_Unlit"))