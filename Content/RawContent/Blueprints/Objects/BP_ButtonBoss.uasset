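; BP_ButtonBoss is an interactable button that completes a boss-area torch puzzle and opens a door.
; On BeginPlay it caches all BP_LightableBoss actors as Torches.
; On Interact, if BP_GuardCharacter's GuardLightsActive count equals the torch count, it opens DoorWay and zeroes that count.
; A puzzle-reset loop that unlights torch materials and lights exists but is never executed.
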(event EventInteract
  (bind _returnvalue (Actor|GetActorOfClass "/Game/ThirdPerson/Blueprints/BP_GuardCharacter.BP_GuardCharacter_C"))
  (if (== (Variables|/Game/ThirdPerson/Blueprints/BP_GuardCharacter.BP_GuardCharacter_C|GetGuardLightsActive _returnvalue) (Utilities|Array|Length (Variables|Default|GetTorches)))
    (Default|DoorOpen (Variables|Default|GetDoorWay))
    (Variables|/Game/ThirdPerson/Blueprints/BP_GuardCharacter.BP_GuardCharacter_C|SetGuardLightsActive _returnvalue 0)))

(event EventBeginPlay
  (bind _outactors (Actor|GetAllActorsOfClass "/Game/RawContent/Blueprints/Objects/BP_LightableBoss.BP_LightableBoss_C"))
  (Variables|Default|SetTorches _outactors))

(fn ConstructionScript)