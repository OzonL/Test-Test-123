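; BP_Bullet is a projectile actor that deals damage to actors it overlaps.
; Tick moves it along its local X axis by a fixed, unswept offset per frame, not scaled by delta time.
; Sphere overlaps filter out certain classes, including other bullets, then send DealDamageMessage through BPI_DealDamage and destroy the bullet.
; Lifespan is set to zero, so bullets that hit no damageable actor never expire.
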(event OnComponentBeginOverlap(Sphere)
  (params (OverlappedComponent :type Primitive%20Component%20Object%20Reference) (OtherActor :type Actor%20Object%20Reference) (OtherComp :type Primitive%20Component%20Object%20Reference) (OtherBodyIndex :type Integer) (bFromSweep :type Boolean) (SweepResult :type Hit%20Result%20Structure%20%28by%20ref%29))
  (bind _returnvalue (Utilities|GetClass OtherActor))
  (if (and (!= _returnvalue 0) (!= _returnvalue "BP_Bullet_C"))
    (if (Utilities|DoesObjectImplementInterface OtherActor "/Game/Interfaces/BPI_DealDamage.BPI_DealDamage_C")
      (Class|BPIDealDamage|DealDamage(Message) OtherActor)
      (Actor|DestroyActor))))

(event EventBeginPlay
  (Variables|Default|SetSpeed "25.000000,0.000000,0.000000")
  (Actor|SetLifeSpan 0.0))

(event EventTick
  (params (DeltaSeconds :type Float%20%28single-precision%29))
  (Transformation|AddActorLocalOffset (Variables|Default|GetSpeed) false false))

(fn ConstructionScript)