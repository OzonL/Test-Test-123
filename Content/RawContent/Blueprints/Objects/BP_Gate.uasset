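; BP_Gate is a gate object that opens or closes whenever its Count reaches two or more.
; Tick polls Count, which nothing in this graph increments, and calls GateToggle at that threshold.
; GateToggle flips the Gate component's visibility, matches collision to it, and resets Count to zero.
; A sound plays at the gate's location only when it becomes visible.
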(event EventTick
  (params (DeltaSeconds :type Float%20%28single-precision%29))
  (if (>= (Variables|Default|GetCount) 2)
    (CallFunction|GateToggle)))

(fn ConstructionScript)

(fn GateToggle
  (bind _gate (Variables|Default|GetGate))
  (Rendering|ToggleVisibility _gate false)
  (if (Variables|/Script/Engine.SceneComponent|GetbVisible _gate)
    (Audio|SpawnSoundatLocation (Variables|Default|GetSFX) (Transformation|GetWorldLocation (Variables|Default|GetGate)) "0, 0, 0" 1.0 1.0 0.0 0 0)
    (Collision|SetCollisionEnabled (Variables|Default|GetGate) "QueryAndPhysics")
    (Variables|Default|SetCount 0)
    (else
      (Collision|SetCollisionEnabled (Variables|Default|GetGate) "NoCollision")
      (Variables|Default|SetCount 0))))