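; BP_Item is a world pickup that spins its mesh, set from item data at construction, and shows text while its sphere is overlapped.
; Interact loops over the BP_GuardCharacter's inventory slots, writing the item into matching stackable or empty slots and breaking after an empty one.
; A write reloads the inventory widget, plays a sound, fires ItemPickup and destroys the actor.
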(event OnComponentBeginOverlap(Sphere)
  (params (OverlappedComponent :type Primitive%20Component%20Object%20Reference) (OtherActor :type Actor%20Object%20Reference) (OtherComp :type Primitive%20Component%20Object%20Reference) (OtherBodyIndex :type Integer) (bFromSweep :type Boolean) (SweepResult :type Hit%20Result%20Structure%20%28by%20ref%29))
  (Development|SetHiddeninGame (Variables|Default|GetTextRender) false false))

(event OnComponentEndOverlap(Sphere)
  (params (OverlappedComponent :type Primitive%20Component%20Object%20Reference) (OtherActor :type Actor%20Object%20Reference) (OtherComp :type Primitive%20Component%20Object%20Reference) (OtherBodyIndex :type Integer))
  (Development|SetHiddeninGame (Variables|Default|GetTextRender) true false))

(event Custom|InventoryBreak
  (bind _item (Variables|Default|GetItem))
  (bind _item_2 (Variables|Default|GetItem))
  (bind (_name _isstackable) (Utilities|Struct|BreakS_ItemStruct _item))
  (Utilities|Array|ForEachLoopwithBreak (Variables|/Game/ThirdPerson/Blueprints/BP_InventoryComponent.BP_InventoryComponent_C|GetItems (Variables|/Game/ThirdPerson/Blueprints/BP_GuardCharacter.BP_GuardCharacter_C|GetBP_InventoryComponent (stale EventBeginPlay _returnvalue)))) ; enters at Break
)

(event EventBeginPlay
  (bind _returnvalue (Actor|GetActorOfClass "/Game/ThirdPerson/Blueprints/BP_GuardCharacter.BP_GuardCharacter_C")))

(event EventTick
  (params (DeltaSeconds :type Float%20%28single-precision%29))
  (Transformation|AddLocalRotation (Variables|Default|GetStaticMesh) (Math|Rotator|MakeRotator 0.0 0.0 (* DeltaSeconds (Variables|Default|GetYawPerSecond))) false false))

(event EventInteract
  (bind _item (Variables|Default|GetItem))
  (bind _item_2 (Variables|Default|GetItem))
  (bind (_name _isstackable) (Utilities|Struct|BreakS_ItemStruct _item))
  (bind (_array_element _array_index) (Utilities|Array|ForEachLoopwithBreak (Variables|/Game/ThirdPerson/Blueprints/BP_InventoryComponent.BP_InventoryComponent_C|GetItems (Variables|/Game/ThirdPerson/Blueprints/BP_GuardCharacter.BP_GuardCharacter_C|GetBP_InventoryComponent (stale EventBeginPlay _returnvalue))))
    (:LoopBody
      (if (and (Utilities|Enum|Equal(Enum) (.Name (Utilities|Struct|BreakS_ItemStruct _array_element)) _name) _isstackable)
        ;[0.15 0.15 0.15 0.5] IF Item Name is not unique and Is Stackable
        (Utilities|Array|SetArrayElem (Variables|/Game/ThirdPerson/Blueprints/BP_InventoryComponent.BP_InventoryComponent_C|GetItems (Variables|/Game/ThirdPerson/Blueprints/BP_GuardCharacter.BP_GuardCharacter_C|GetBP_InventoryComponent (stale EventBeginPlay _returnvalue))) _array_index (Utilities|Struct|MakeS_ItemStruct (.name _item_2) (.isstackable _item_2) (.amount _item_2) (.thumbnail _item_2) (.staticmesh _item_2)))
        (Default|LoadInventory (Variables|/Game/ThirdPerson/Blueprints/BP_InventoryComponent.BP_InventoryComponent_C|GetInventoryWidget (Variables|/Game/ThirdPerson/Blueprints/BP_GuardCharacter.BP_GuardCharacter_C|GetBP_InventoryComponent (stale EventBeginPlay _returnvalue))) (Variables|/Game/ThirdPerson/Blueprints/BP_GuardCharacter.BP_GuardCharacter_C|GetBP_InventoryComponent (stale EventBeginPlay _returnvalue)) :!label _label)
        (Audio|PlaySound2D (Variables|Default|GetSFX) 1.0 1.0 0.0 0 0)
        (Default|CallItemPickup)
        (Actor|DestroyActor)
        (else
          ;[0.15 0.15 0.15 0.5] IF Item Name is unique:
          (if (== (.Amount (Utilities|Struct|BreakS_ItemStruct _array_element)) 0)
            (Utilities|Array|SetArrayElem (Variables|/Game/ThirdPerson/Blueprints/BP_InventoryComponent.BP_InventoryComponent_C|GetItems (Variables|/Game/ThirdPerson/Blueprints/BP_GuardCharacter.BP_GuardCharacter_C|GetBP_InventoryComponent (stale EventBeginPlay _returnvalue))) _array_index (Variables|Default|GetItem))
            (CallFunction|InventoryBreak)
            (goto _label)))))))

(fn ConstructionScript
  (Components|StaticMesh|SetStaticMesh (Variables|Default|GetStaticMesh) (.StaticMesh (Utilities|Struct|BreakS_ItemStruct (Variables|Default|GetItem)))))