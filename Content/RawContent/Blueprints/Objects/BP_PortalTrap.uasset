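; Portal actor that loads the level set in LevelName when something overlaps its trigger box while IsActive is true.
; On BeginPlay, an inactive portal switches off several named emitters of its Niagara effect, NSPortal04.
; An overlap on an active portal plays a 2D portal sound and opens the level after a short delay, with no check on the overlapping actor.
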(event OnComponentBeginOverlap(Box)
  (params (OverlappedComponent :type Primitive%20Component%20Object%20Reference) (OtherActor :type Actor%20Object%20Reference) (OtherComp :type Primitive%20Component%20Object%20Reference) (OtherBodyIndex :type Integer) (bFromSweep :type Boolean) (SweepResult :type Hit%20Result%20Structure%20%28by%20ref%29))
  (if (Variables|Default|GetIsActive)
    (Audio|PlaySound2D "/Game/RawContent/Sounds/portal.portal" 1.0 1.0 0.0 0 0)
    (Utilities|FlowControl|Delay 2.0)
    (Game|OpenLevel(byName) (Variables|Default|GetLevelName))))

(event EventBeginPlay
  (bind _ns_portal_04 (Variables|Default|GetNS_Portal_04))
  (if (not (Variables|Default|GetIsActive))
    (Effects|Components|ParticleSystem|SetEmitterEnable _ns_portal_04 "Swirl" false)
    (Effects|Components|ParticleSystem|SetEmitterEnable _ns_portal_04 "SparksRing" false)
    (Effects|Components|ParticleSystem|SetEmitterEnable _ns_portal_04 "ground" false)
    (Effects|Components|ParticleSystem|SetEmitterEnable _ns_portal_04 "ground002" false)
    (Effects|Components|ParticleSystem|SetEmitterEnable _ns_portal_04 "parts003" false)
    (Effects|Components|ParticleSystem|SetEmitterEnable _ns_portal_04 "parts002" false)))

(fn ConstructionScript)