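; Puzzle statue that tracks the guard character and, once activated, lights its button and counts toward a linked gate.
; A Number variable selects one of four unlit button colours at BeginPlay.
; Any Box overlap while the guard's Box collision is QueryAndPhysics activates it once, incrementing the gate's Count.
; Sphere overlaps set the target; Tick smoothly yaws toward a guard target while the gate is visible and the statue inactive.
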(event OnComponentBeginOverlap(Box)
  (params (OverlappedComponent :type Primitive%20Component%20Object%20Reference) (OtherActor :type Actor%20Object%20Reference) (OtherComp :type Primitive%20Component%20Object%20Reference) (OtherBodyIndex :type Integer) (bFromSweep :type Boolean) (SweepResult :type Hit%20Result%20Structure%20%28by%20ref%29))
  (bind _returnvalue (Actor|GetActorOfClass "/Game/ThirdPerson/Blueprints/BP_GuardCharacter.BP_GuardCharacter_C"))
  (if (Utilities|Enum|Equal(Enum) (Collision|GetCollisionEnabled (Variables|/Game/ThirdPerson/Blueprints/BP_GuardCharacter.BP_GuardCharacter_C|GetBox _returnvalue)) "QueryAndPhysics")
    (Utilities|FlowControl|DoOnce false
      (:Completed
        (Rendering|Material|SetMaterial (Variables|Default|GetButton) 0 (Variables|Default|GetMaterial))
        (Variables|Default|SetActivated true)
        (bind _result (Math|Integer|IncrementInt (Variables|/Game/RawContent/Blueprints/Objects/BP_Gate.BP_Gate_C|GetCount (Variables|Default|GetGate)))
          (:%20%20
            (Variables|/Game/RawContent/Blueprints/Objects/BP_Gate.BP_Gate_C|SetCount (Variables|Default|GetGate) _result)))))))

(event OnComponentBeginOverlap(Sphere)
  (params (OverlappedComponent :type Primitive%20Component%20Object%20Reference) (OtherActor :type Actor%20Object%20Reference) (OtherComp :type Primitive%20Component%20Object%20Reference) (OtherBodyIndex :type Integer) (bFromSweep :type Boolean) (SweepResult :type Hit%20Result%20Structure%20%28by%20ref%29))
  (Variables|Default|SetTargetActor OtherActor))

(event EventTick
  (params (DeltaSeconds :type Float%20%28single-precision%29))
  (if (Math|Boolean|ANDBoolean (== (Utilities|GetClass (Variables|Default|GetTargetActor)) "/Game/ThirdPerson/Blueprints/BP_GuardCharacter.BP_GuardCharacter_C") (Rendering|IsVisible (Variables|/Game/RawContent/Blueprints/Objects/BP_Gate.BP_Gate_C|GetGate (Variables|Default|GetGate))) (not (Variables|Default|GetActivated)))
    (CallFunction|RotateTowardsPlayer DeltaSeconds (Variables|Default|GetTargetActor))))

(event EventBeginPlay
  (bind _number (Variables|Default|GetNumber))
  (if (== _number 0)
    (Variables|Default|SetMaterial "/Game/Materials/M_PurpleUnlit.M_PurpleUnlit")
    (elif (== _number 1)
      (Variables|Default|SetMaterial "/Game/Materials/M_GreenUnlit.M_GreenUnlit")
      (elif (== _number 2)
        (Variables|Default|SetMaterial "/Game/Materials/M_BlueUnlit.M_BlueUnlit")
        (elif (== _number 3)
          (Variables|Default|SetMaterial "/Game/Materials/M_RedUnlit.M_RedUnlit"))))))

(fn ConstructionScript)

(fn RotateTowardsPlayer
  (params (DeltaTime :type Float%20%28double-precision%29) (TargetActor :type Actor%20Object%20Reference))
  (bind _returnvalue (Transformation|GetActorRotation))
  (Transformation|SetActorRotation (Math|Rotator|MakeRotator (.roll _returnvalue) (.pitch _returnvalue) (.yaw (Math|Rotator|Lerp(Rotator) (Math|Rotator|MakeRotator 0.0 0.0 (.yaw _returnvalue)) (Math|Rotator|MakeRotator 0.0 0.0 (.yaw (Math|Rotator|FindLookatRotation (Transformation|GetActorLocation) (Transformation|GetActorLocation TargetActor)))) (* DeltaTime 1.5) true)))))