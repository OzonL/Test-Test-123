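; BP_Item is an interactable pickup actor whose construction script sets its mesh from its Item struct.
; On Interact it loops over the guard character's inventory component, overwriting a matching stackable slot with its own values, without summing amounts, or filling an empty slot.
; A non-matching slot ends the loop through InventoryBreak, whether filled or not.
; A successful write reloads the inventory widget and destroys the actor.
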(event Custom|InventoryBreak
  (bind _item (Variables|Default|GetItem))
  (bind _item_2 (Variables|Default|GetItem))
  (bind (_name _isstackable) (Utilities|Struct|BreakS_ItemStruct _item))
  (Utilities|Array|ForEachLoopwithBreak (Variables|/Game/ThirdPerson/Blueprints/BP_InventoryComponent.BP_InventoryComponent_C|GetItems (Variables|/Game/ThirdPerson/Blueprints/BP_GuardCharacter.BP_GuardCharacter_C|GetBP_InventoryComponent (stale EventBeginPlay _returnvalue)))) ; enters at Break
)

(event EventBeginPlay
  (bind _returnvalue (Actor|GetActorOfClass "/Game/ThirdPerson/Blueprints/BP_GuardCharacter.BP_GuardCharacter_C")))

(event EventInteract
  (bind _item (Variables|Default|GetItem))
  (bind _item_2 (Variables|Default|GetItem))
  (bind (_name _isstackable) (Utilities|Struct|BreakS_ItemStruct _item))
  (bind (_array_element _array_index) (Utilities|Array|ForEachLoopwithBreak (Variables|/Game/ThirdPerson/Blueprints/BP_InventoryComponent.BP_InventoryComponent_C|GetItems (Variables|/Game/ThirdPerson/Blueprints/BP_GuardCharacter.BP_GuardCharacter_C|GetBP_InventoryComponent (stale EventBeginPlay _returnvalue))))
    (:LoopBody
      (if (and (Utilities|Enum|Equal(Enum) (.Name (Utilities|Struct|BreakS_ItemStruct _array_element)) _name) _isstackable)
        (Utilities|Array|SetArrayElem (Variables|/Game/ThirdPerson/Blueprints/BP_InventoryComponent.BP_InventoryComponent_C|GetItems (Variables|/Game/ThirdPerson/Blueprints/BP_GuardCharacter.BP_GuardCharacter_C|GetBP_InventoryComponent (stale EventBeginPlay _returnvalue))) _array_index (Utilities|Struct|MakeS_ItemStruct (.name _item_2) (.isstackable _item_2) (.amount _item_2) (.thumbnail _item_2) (.staticmesh _item_2)))
        (Default|LoadInventory (Variables|/Game/ThirdPerson/Blueprints/BP_InventoryComponent.BP_InventoryComponent_C|GetInventoryWidget (Variables|/Game/ThirdPerson/Blueprints/BP_GuardCharacter.BP_GuardCharacter_C|GetBP_InventoryComponent (stale EventBeginPlay _returnvalue))) (Variables|/Game/ThirdPerson/Blueprints/BP_GuardCharacter.BP_GuardCharacter_C|GetBP_InventoryComponent (stale EventBeginPlay _returnvalue)) :!label _label)
        (Actor|DestroyActor)
        (elif (== (.Amount (Utilities|Struct|BreakS_ItemStruct _array_element)) 0)
          (Utilities|Array|SetArrayElem (Variables|/Game/ThirdPerson/Blueprints/BP_InventoryComponent.BP_InventoryComponent_C|GetItems (Variables|/Game/ThirdPerson/Blueprints/BP_GuardCharacter.BP_GuardCharacter_C|GetBP_InventoryComponent (stale EventBeginPlay _returnvalue))) _array_index (Variables|Default|GetItem))
          (CallFunction|InventoryBreak)
          (goto _label)
          (else
            (CallFunction|InventoryBreak)))))))

(fn ConstructionScript
  (Components|StaticMesh|SetStaticMesh (Variables|Default|GetStaticMesh) (.StaticMesh (Utilities|Struct|BreakS_ItemStruct (Variables|Default|GetItem)))))