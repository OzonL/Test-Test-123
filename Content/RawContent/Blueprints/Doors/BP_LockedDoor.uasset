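; BP_LockedDoor is a door that stays shut until its key is picked up, then opens when an actor enters its trigger box.
; While it is locked, overlapping the box shows a text message, which hides on exit.
; The Key's ItemPickup event clears IsLocked, letting the Dooranim timeline slide the door mesh along local Y and reverse on exit.
; Any overlapping actor triggers it, as the guard class check is unused.
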(event OnComponentBeginOverlap(Box)
  (params (OverlappedComponent :type Primitive%20Component%20Object%20Reference) (OtherActor :type Actor%20Object%20Reference) (OtherComp :type Primitive%20Component%20Object%20Reference) (OtherBodyIndex :type Integer) (bFromSweep :type Boolean) (SweepResult :type Hit%20Result%20Structure%20%28by%20ref%29))
  (if (Variables|Default|GetIsLocked)
    (Rendering|SetVisibility (Variables|Default|GetTextRender) true false)
    (else
      ;[0.15 0.15 0.15 0.5] Open/Close Door
      (bind _doorswing (Timeline|Dooranim Play)
        (:Update
          (Transformation|SetRelativeLocation (Variables|Default|GetSM_Door1) (Math|Vector|MakeVector 0.0 (Math|Float|Lerp 0.0 9e+01 _doorswing) 0.0) false false))))))

(event OnComponentEndOverlap(Box)
  (params (OverlappedComponent :type Primitive%20Component%20Object%20Reference) (OtherActor :type Actor%20Object%20Reference) (OtherComp :type Primitive%20Component%20Object%20Reference) (OtherBodyIndex :type Integer))
  (bind _textrender (Variables|Default|GetTextRender))
  (if (Rendering|IsVisible _textrender)
    (Rendering|SetVisibility _textrender false false)
    (else
      ;[0.15 0.15 0.15 0.5] Open/Close Door
      (bind _doorswing (Timeline|Dooranim Reverse)
        (:Update
          (Transformation|SetRelativeLocation (Variables|Default|GetSM_Door1) (Math|Vector|MakeVector 0.0 (Math|Float|Lerp 0.0 9e+01 _doorswing) 0.0) false false))))))

(event ItemPickup(Key)
  (Variables|Default|SetIsLocked false))

(fn ConstructionScript)