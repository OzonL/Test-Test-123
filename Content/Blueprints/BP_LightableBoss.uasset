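; BP_LightableBoss is an interactable light that forms one step of an ordered lighting puzzle.
; On Interact, if it is unlit and the cached BP_GuardCharacter has a torch equipped, it shows its PointLight and applies the lit cube material.
; It increments the guard's GuardLightsActive counter when that matches its SequenceNumber, otherwise zeroes it.
; Reset hides only the light, leaving the material unchanged.
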(event EventInteract
  (bind _pointlight (Variables|Default|GetPointLight))
  (if (not (Rendering|IsVisible _pointlight))
    (if (Variables|/Game/ThirdPerson/Blueprints/BP_GuardCharacter.BP_GuardCharacter_C|GetTorchIsEquipped (stale EventBeginPlay _returnvalue))
      (Rendering|SetVisibility _pointlight true false)
      (Rendering|Material|SetMaterial (Variables|Default|GetCube) 0 "/Game/Materials/M_Lit.M_Lit")
      (if (== (Variables|/Game/ThirdPerson/Blueprints/BP_GuardCharacter.BP_GuardCharacter_C|GetGuardLightsActive (stale EventBeginPlay _returnvalue)) (Variables|Default|GetSequenceNumber))
        (bind _returnvalue (Actor|GetActorOfClass "/Game/ThirdPerson/Blueprints/BP_GuardCharacter.BP_GuardCharacter_C"))
        (bind _result (Math|Integer|IncrementInt (Variables|/Game/ThirdPerson/Blueprints/BP_GuardCharacter.BP_GuardCharacter_C|GetGuardLightsActive _returnvalue))
          (:%20%20
            (bind _output_get (Variables|/Game/ThirdPerson/Blueprints/BP_GuardCharacter.BP_GuardCharacter_C|SetGuardLightsActive _returnvalue _result))
            (Development|PrintString (Utilities|String|ToString(Integer) _output_get))))
        (else
          (bind _returnvalue_2 (Actor|GetActorOfClass "/Game/ThirdPerson/Blueprints/BP_GuardCharacter.BP_GuardCharacter_C"))
          (Variables|/Game/ThirdPerson/Blueprints/BP_GuardCharacter.BP_GuardCharacter_C|SetGuardLightsActive _returnvalue_2 0))))))

(event EventBeginPlay
  (bind _returnvalue (Actor|GetActorOfClass "/Game/ThirdPerson/Blueprints/BP_GuardCharacter.BP_GuardCharacter_C")))

(fn ConstructionScript)

(fn Reset
  (Rendering|SetVisibility (Variables|Default|GetPointLight) false false))