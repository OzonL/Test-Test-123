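; Boss enemy that hunts the BP_GuardCharacter and destroys itself once that character's GuardLightsActive count reaches four.
; Each Tick it turns to face the guard and, while the guard is outside its Radius component, eases toward them on XY at constant height.
; A one-second Delay in that same Tick branch throttles BP_Bullet spawns at the boss's transform.
; Radius overlap events toggle InRadius, halting pursuit and new shots when the guard is close.
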(event OnComponentBeginOverlap(Radius)
  (params (OverlappedComponent :type Primitive%20Component%20Object%20Reference) (OtherActor :type Actor%20Object%20Reference) (OtherComp :type Primitive%20Component%20Object%20Reference) (OtherBodyIndex :type Integer) (bFromSweep :type Boolean) (SweepResult :type Hit%20Result%20Structure%20%28by%20ref%29))
  (if (== (Utilities|GetClass OtherActor) "/Game/ThirdPerson/Blueprints/BP_GuardCharacter.BP_GuardCharacter_C")
    (Variables|Default|SetInRadius true)))

(event OnComponentEndOverlap(Radius)
  (params (OverlappedComponent :type Primitive%20Component%20Object%20Reference) (OtherActor :type Actor%20Object%20Reference) (OtherComp :type Primitive%20Component%20Object%20Reference) (OtherBodyIndex :type Integer))
  (if (== (Utilities|GetClass OtherActor) "/Game/ThirdPerson/Blueprints/BP_GuardCharacter.BP_GuardCharacter_C")
    (Variables|Default|SetInRadius false)))

(event EventBeginPlay
  (Variables|Default|SetInRadius false))

(event Collision|EventActorBeginOverlap
  (params (OtherActor :type Actor%20Object%20Reference)))

(event EventTick
  (params (DeltaSeconds :type Float%20%28single-precision%29))
  (bind _returnvalue (Actor|GetActorOfClass "/Game/ThirdPerson/Blueprints/BP_GuardCharacter.BP_GuardCharacter_C"))
  (if (== (Variables|/Game/ThirdPerson/Blueprints/BP_GuardCharacter.BP_GuardCharacter_C|GetGuardLightsActive _returnvalue) 4)
    (Actor|DestroyActor)
    (else
      (CallFunction|RotateTowardsPlayer)
      (if (not (Variables|Default|GetInRadius))
        (CallFunction|PlayerFollow DeltaSeconds)
        (Utilities|FlowControl|Delay (Math|Random|RandomFloatinRange 1.0 1.0))
        (CallFunction|FireatPlayer)))))

(fn ConstructionScript)

(fn RotateTowardsPlayer
  (bind _returnvalue (Actor|GetActorOfClass "/Game/ThirdPerson/Blueprints/BP_GuardCharacter.BP_GuardCharacter_C"))
  (Transformation|SetActorRotation (Math|Rotator|FindLookatRotation (Transformation|GetActorLocation) (Transformation|GetActorLocation _returnvalue))))

(fn FireatPlayer
  (Game|SpawnActorfromClass "/Game/RawContent/Blueprints/Objects/BP_Bullet.BP_Bullet_C" (Transformation|GetActorTransform) "AlwaysSpawn" "MultiplyWithRoot" 0 0))

(fn PlayerFollow
  (params (deltaTime :type Float%20%28double-precision%29))
  (bind _returnvalue (Transformation|GetActorLocation))
  (bind _returnvalue_2 (Actor|GetActorOfClass "/Game/ThirdPerson/Blueprints/BP_GuardCharacter.BP_GuardCharacter_C"))
  (Transformation|SetActorLocation (Math|Interpolation|VInterpTo (Math|Vector|MakeVector (.x _returnvalue) (.y _returnvalue) (.z _returnvalue)) (Math|Vector|MakeVector (.x (Transformation|GetActorLocation _returnvalue_2)) (.y (Transformation|GetActorLocation _returnvalue_2)) (.z _returnvalue)) deltaTime 0.5) true false))