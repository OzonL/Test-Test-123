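; BP_Win is the interactable win check for a torch puzzle.
; On Interact it compares the BP_GuardCharacter's GuardLightsActive with the length of the Torches array, and on a match unhides the first TextRenderActor found.
; Otherwise it resets each torch to the unlit material and hides its point light and fire effect, leaving the guard's count untouched.
; BeginPlay runs an actor search but shows Torches set to None.
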(event EventInteract
  (bind _torches (Variables|Default|GetTorches))
  (bind _returnvalue (Actor|GetActorOfClass "/Game/ThirdPerson/Blueprints/BP_GuardCharacter.BP_GuardCharacter_C"))
  (if (== (Variables|/Game/ThirdPerson/Blueprints/BP_GuardCharacter.BP_GuardCharacter_C|GetGuardLightsActive _returnvalue) (Utilities|Array|Length _torches))
    (bind _returnvalue_2 (Actor|GetActorOfClass "/Script/Engine.TextRenderActor"))
    (Rendering|SetActorHiddenInGame _returnvalue_2 false)
    (else
      ;[0.15 0.15 0.15 0.5] Reset Puzzle
      (for _array_element _torches
        (Rendering|Material|SetMaterial (Variables|Default|GetLamp _array_element) 1 "/Game/Materials/M_Unlit.M_Unlit")
        (Rendering|SetVisibility (Variables|Default|GetPointLight _array_element) false false)
        (Rendering|SetVisibility (Variables|Default|GetNS_Stylish_Fire_4 _array_element) false false)))))

(event EventBeginPlay
  (bind _outactors (Actor|GetAllActorsOfClass 0))
  (Variables|Default|SetTorches 0 _outactors))

(fn ConstructionScript)