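; BP_Button is an interactable puzzle button that opens a linked doorway once every torch is lit.
; On BeginPlay it caches all BP_Lightable actors as torches.
; On Interact it compares the LightsActivated count on BP_ThirdPersonCharacter with the torch count and opens DoorWay on a match.
; Otherwise it visually unlights every torch through material and light visibility, leaving the character's count untouched.
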(event EventInteract
  (bind _torches (Variables|Default|GetTorches))
  (bind _returnvalue (Actor|GetActorOfClass "/Game/ThirdPerson/Blueprints/BP_ThirdPersonCharacter.BP_ThirdPersonCharacter_C"))
  (if (== (Variables|/Game/ThirdPerson/Blueprints/BP_ThirdPersonCharacter.BP_ThirdPersonCharacter_C|GetLightsActivated _returnvalue) (Utilities|Array|Length _torches))
    (Default|DoorOpen (Variables|Default|GetDoorWay))
    (else
      ;[0.15 0.15 0.15 0.5] Reset Puzzle
      (for _array_element _torches
        (Rendering|Material|SetMaterial (Variables|/Game/Blueprints/BP_Lightable.BP_Lightable_C|GetLamp _array_element) 1 "/Game/Materials/M_Unlit.M_Unlit")
        (Rendering|SetVisibility (Variables|/Game/Blueprints/BP_Lightable.BP_Lightable_C|GetPointLight _array_element) false false)))))

(event EventBeginPlay
  (bind _outactors (Actor|GetAllActorsOfClass "/Game/Blueprints/BP_Lightable.BP_Lightable_C"))
  (Variables|Default|SetTorches _outactors))

(fn ConstructionScript)