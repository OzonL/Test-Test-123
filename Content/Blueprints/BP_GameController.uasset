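; Game controller Blueprint that starts the BossTheme music and handles the end-game fade-out.
; BeginPlay clears the EndGame flag, then creates and plays the theme as a 2D sound.
; While EndGame is true, which nothing here sets, every Tick adds a new BP_FadeOut widget to the viewport and replays the theme if it has stopped.
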(event EventBeginPlay
  (Variables|Default|SetEndGame false)
  (bind _returnvalue (Audio|CreateSound2D "/Game/RawContent/Sounds/BossTheme.BossTheme" 1.0 1.0 0.0 0))
  (Audio|Components|Audio|Play _returnvalue 0.0))

(event Collision|EventActorBeginOverlap
  (params (OtherActor :type Actor%20Object%20Reference)))

(event EventTick
  (params (DeltaSeconds :type Float%20%28single-precision%29))
  (if (Variables|Default|GetEndGame)
    (bind _returnvalue (UserInterface|CreateWidget "/Game/Blueprints/BP_FadeOut.BP_FadeOut_C"))
    (UserInterface|Viewport|AddtoViewport _returnvalue 0)
    (if (not (Audio|Components|Audio|IsPlaying (stale EventBeginPlay _returnvalue)))
      (Audio|Components|Audio|Play (stale EventBeginPlay _returnvalue) 0.0))))

(fn ConstructionScript)